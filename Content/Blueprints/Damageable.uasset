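; Damageable Blueprint that tracks a Life value and signals death when damage depletes it.
; GetDamage takes a damage amount and updates Life through math expression nodes, apparently subtracting the amount and testing for zero or below.
; When that check passes, it calls the Die dispatcher, leaving the death response outside this graph.
; BeginPlay and Tick are empty, so the logic runs only when GetDamage is called.
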(event EventBeginPlay)

(event EventTick
  (params (DeltaSeconds :type Float%20%28single-precision%29)))

(fn GetDamage
  (params (Taken :type Float%20%28single-precision%29))
  (Variables|Game|SetLife (|({2107B857-031F-4CA8-B305-3F1A1DF321CF}-Taken) Taken))
  (if (|({2107B857-031F-4CA8-B305-3F1A1DF321CF}<=0))
    (Default|CallDie)))