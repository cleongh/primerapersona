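; ShootTask is an AI task that has an Enemy damage the player's FirstPersonCharacter when within a distance threshold.
; On each AI tick in range it counts down an attack timer, and at zero applies the Enemy's DamageDone directly, without a projectile or trace, then resets the timer.
; It finishes successfully on any in-range tick, even while cooling down, and fails when the player is out of range.
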(event `self.ReceiveTickAI`
  (params (OwnerController :type "AIController Object Reference") (ControlledPawn :type "Pawn Object Reference") (DeltaSeconds :type "Float (single-precision)"))
  (bind _asfirst_person_character (cast `/Game/Blueprints/FirstPersonCharacter` (`GameplayStatics.GetPlayerPawn` 0)))
  (if (< (`Actor.GetDistanceTo` ControlledPawn _asfirst_person_character) (`self.Distance threshold`))
    (bind _output_get (set `self.Attack counter` (`KismetMathLibrary.FMax` (- (`self.Attack counter`) DeltaSeconds))))
    (if (<= _output_get 0.0)
      (bind _asenemy (cast `/Game/Blueprints/Enemy` ControlledPawn))
      (`GameplayStatics.ApplyDamage` _asfirst_person_character (`/Game/Blueprints/Enemy.Damage done` _asenemy) null ControlledPawn)
      (set `self.Attack counter` (`self.Attack period`)))
    (`self.FinishExecute` true)
    (else
      (`self.FinishExecute` false))))