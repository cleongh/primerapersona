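; Zombie enemy Blueprint that takes damage from first-person projectiles and is destroyed when it dies.
; On a projectile hit, it looks up the player character's current weapon in a damage map and passes that value to its Damageable component.
; It binds the component's Die event at BeginPlay to destroy itself.
; A leftover, disconnected branch for damaging a top-down player never runs.
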(event `self.ReceiveBeginPlay`
  (`parent.ReceiveBeginPlay`)
  (add `/Game/Blueprints/Damageable.Die` (`self.Damageable`) (delegate `Die_Event_0`)))

(event `Die_Event_0`
  (`self.K2_DestroyActor`))

(event `self.ReceiveHit`
  (params (MyComp :type "PrimitiveComponent Object Reference") (Other :type "Actor Object Reference") (OtherComp :type "PrimitiveComponent Object Reference") (bSelfMoved :type Boolean) (HitLocation :type "Vector Structure") (HitNormal :type "Vector Structure") (NormalImpulse :type "Vector Structure") (Hit :type "HitResult Structure (by ref)"))
  (cast `/Game/Blueprints/FirstPersonProjectile` Other)
  (bind _asfirst_person_character (cast `/Game/Blueprints/FirstPersonCharacter` (`GameplayStatics.GetPlayerPawn` 0)))
  (`/Game/Blueprints/Damageable.Get damage` (`self.Damageable`) (`BlueprintMapLibrary.Map_Find` (`/Game/Blueprints/FirstPersonCharacter.WeaponDamage` _asfirst_person_character) (`/Game/Blueprints/FirstPersonCharacter.Current` _asfirst_person_character))))

(fn `UserConstructionScript`
  (`parent.UserConstructionScript`))